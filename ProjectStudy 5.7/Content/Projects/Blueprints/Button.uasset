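; Floor button Blueprint that opens a linked TargetDoor when the player steps into its trigger box.
; A BP_Player overlap plays the SwitchOn timeline, which animates the button mesh's relative location.
; When the timeline ends and the door is valid, it opens the door and calls SetEventFinished.
; That override calls the parent, sets the button's relative location to zero and disables box collision, retiring the trigger.
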(event OnComponentBeginOverlap(Box)
  (params (OverlappedComponent :type Primitive%20Component%20Object%20Reference) (OtherActor :type Actor%20Object%20Reference) (OtherComp :type Primitive%20Component%20Object%20Reference) (OtherBodyIndex :type Integer) (bFromSweep :type Boolean) (SweepResult :type Hit%20Result%20Structure%20%28by%20ref%29))
  (Utilities|Casting|CastToBP_Player OtherActor)
  (bind _buttonz (Timeline|SwitchOn Play)
    (:Update
      (Transformation|SetRelativeLocation (Variables|コンポーネント|GetButton) (Math|Conversions|ToVector(Float) _buttonz) false false))
    (:Finished
      (bind _targetdoor (Variables|Default|GetTargetDoor)
        (:then
          (Default|OpenDoor _targetdoor)
          (CallFunction|SetEventFinished))
        (:else)))))

(event EventBeginPlay
  (|CallParentFunction))

(fn ConstructionScript)

(fn SetEventFinished
  (|CallParentFunction)
  (Transformation|SetRelativeLocation (Variables|コンポーネント|GetButton) "0, 0, 0" false false)
  (Collision|SetCollisionEnabled (Variables|コンポーネント|GetBox) "NoCollision"))