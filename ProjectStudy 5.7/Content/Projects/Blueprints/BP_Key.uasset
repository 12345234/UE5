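; BP_Key is a key pickup that spins in the level and disappears when the player touches it.
; A Rotation timeline, started on BeginPlay, drives the yaw of the key mesh.
; On sphere overlap with BP_Player, it saves a new status for its KeyName through the game instance, then calls SetEventFinished.
; That override runs the inherited event-finish logic and destroys the actor.
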(event OnComponentBeginOverlap(Sphere)
  (params (OverlappedComponent :type Primitive%20Component%20Object%20Reference) (OtherActor :type Actor%20Object%20Reference) (OtherComp :type Primitive%20Component%20Object%20Reference) (OtherBodyIndex :type Integer) (bFromSweep :type Boolean) (SweepResult :type Hit%20Result%20Structure%20%28by%20ref%29))
  ;[0.15 0.15 0.15 0.5] 当たり判定(プレイヤーに当たると消える)
  (Utilities|Casting|CastToBP_Player OtherActor)
  (Default|SaveKeyStatus (Variables|Default|GetMyGameInstance) (Variables|Default|GetKeyName) "NewEnumerator1")
  (CallFunction|SetEventFinished))

(event EventBeginPlay
  (bind _stm_key (Variables|Default|GetSTM_Key))
  (bind _relativerotation (Variables|/Script/Engine.SceneComponent|GetRelativeRotation _stm_key))
  (bind (_roll _pitch) (Math|Rotator|BreakRotator _relativerotation))
  ;[0.15 0.15 0.15 0.5] オブジェクトの回転
  (|CallParentFunction)
  (bind _rotationz (Timeline|Rotation Play)
    (:Update
      (Transformation|SetRelativeRotation (Variables|Default|GetSTM_Key) (Math|Rotator|MakeRotator _roll _pitch _rotationz) false false))))

(fn ConstructionScript)

(fn SetEventFinished
  (|CallParentFunction)
  (Actor|DestroyActor))