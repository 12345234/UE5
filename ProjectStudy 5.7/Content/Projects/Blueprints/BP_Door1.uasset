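; BP_Door1 is a door that opens when the player overlaps its trigger box, optionally requiring a key.
; Unlocked doors open immediately; otherwise the key must have Got status in the game instance, which is then reset to Default.
; Opening destroys the actor and calls SetEventFinished, an extension of the parent function that clears SwitchDoor, rotates the door mesh and disables box collision.
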(event OnComponentBeginOverlap(Box)
  (params (OverlappedComponent :type Primitive%20Component%20Object%20Reference) (OtherActor :type Actor%20Object%20Reference) (OtherComp :type Primitive%20Component%20Object%20Reference) (OtherBodyIndex :type Integer) (bFromSweep :type Boolean) (SweepResult :type Hit%20Result%20Structure%20%28by%20ref%29))
  (Utilities|Casting|CastToBP_Player OtherActor)
  (if (and (== (Variables|Default|GetKeyName) "") (not (Variables|Default|GetSwitchDoor)))
    (CallFunction|OpenDoor1)
    (else
      (switch Utilities|FlowControl|Switch|SwitchonEN_KeyStatus (Default|GetKeyStatus (Variables|Default|GetMyGameInstance) (Variables|Default|GetKeyName))
        (:NewEnumerator1
          (Default|SaveKeyStatus (Variables|Default|GetMyGameInstance) (Variables|Default|GetKeyName) "NewEnumerator0")
          (CallFunction|OpenDoor1))))))

(event Custom|OpenDoor1
  (Variables|Default|SetSwitchDoor false)
  (Actor|DestroyActor self)
  (CallFunction|SetEventFinished))

(event EventBeginPlay
  (|CallParentFunction))

(fn ConstructionScript)

(fn SetEventFinished
  (|CallParentFunction)
  (Variables|Default|SetSwitchDoor false)
  (Transformation|SetRelativeRotation (Variables|コンポーネント|GetSTM_Door) "0.000000,-90.000000,0.000000" false false)
  (Collision|SetCollisionEnabled (Variables|コンポーネント|GetBox) "NoCollision"))