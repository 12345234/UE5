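; Player character with Enhanced Input look, move and jump that can pull levers and restarts the current level when destroyed.
; Creates the game UI and seeds key statuses from a DataTable into the game instance if empty.
; Capsule overlaps track the current actor, driving lever interaction and door or lever prompts based on key state.
; Overridden death and goal events update the UI's corresponding messages.
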(event OnComponentBeginOverlap(CapsuleComponent)
  (params (OverlappedComponent :type Primitive%20Component%20Object%20Reference) (OtherActor :type Actor%20Object%20Reference) (OtherComp :type Primitive%20Component%20Object%20Reference) (OtherBodyIndex :type Integer) (bFromSweep :type Boolean) (SweepResult :type Hit%20Result%20Structure%20%28by%20ref%29))
  (Variables|Default|SetOverlapActor OtherActor)
  (CallFunction|UpdateMessage))

(event OnComponentEndOverlap(CapsuleComponent)
  (params (OverlappedComponent :type Primitive%20Component%20Object%20Reference) (OtherActor :type Actor%20Object%20Reference) (OtherComp :type Primitive%20Component%20Object%20Reference) (OtherBodyIndex :type Integer))
  (Variables|Default|SetOverlapActor 0)
  (CallFunction|UpdateMessage))

(event Input|EnhancedActionEvents|EnhancedInputActionIA_MyLook
  (params (ActionValue :type Vector%202D%20Structure) (ElapsedSeconds :type Float%20%28double-precision%29) (TriggeredSeconds :type Float%20%28double-precision%29) (InputAction :type Input%20Action%20Object%20Reference :default "/Game/Projects/IA_MyLook.IA_MyLook"))
  (Pawn|Input|AddControllerYawInput (.x ActionValue))
  (Pawn|Input|AddControllerPitchInput (.y ActionValue)))

(event Input|EnhancedActionEvents|EnhancedInputActionIA_MyMove
  (params (ActionValue :type Vector%202D%20Structure) (ElapsedSeconds :type Float%20%28double-precision%29) (TriggeredSeconds :type Float%20%28double-precision%29) (InputAction :type Input%20Action%20Object%20Reference :default "/Game/Projects/IA_MyMove.IA_MyMove"))
  (Utilities|FlowControl|Sequence
    (:then_0
      (Pawn|Input|AddMovementInput (Math|Vector|GetRightVector (Pawn|GetControlRotation :!class /Script/Engine.Pawn)) (.x ActionValue) false))
    (:then_1
      (Pawn|Input|AddMovementInput (Math|Vector|GetForwardVector (Pawn|GetControlRotation :!class /Script/Engine.Pawn)) (.y ActionValue) false))))

(event Input|EnhancedActionEvents|EnhancedInputActionIA_MyJump
  (params (ActionValue :type Boolean) (ElapsedSeconds :type Float%20%28double-precision%29) (TriggeredSeconds :type Float%20%28double-precision%29) (InputAction :type Input%20Action%20Object%20Reference :default "/Game/Projects/IA_MyJump.IA_MyJump"))
  (:Started
    (Character|Jump))
  (:Completed
    (Character|StopJumping)))

(event Input|EnhancedActionEvents|EnhancedInputActionIA_MyAccessEvent
  (params (ActionValue :type Boolean) (ElapsedSeconds :type Float%20%28double-precision%29) (TriggeredSeconds :type Float%20%28double-precision%29) (InputAction :type Input%20Action%20Object%20Reference :default "/Game/Projects/IA_MyAccessEvent.IA_MyAccessEvent"))
  (:Started
    (bind _overlapactor (Variables|Default|GetOverlapActor)
      (:then
        (bind _asbp_lever (Utilities|Casting|CastToBP_Lever _overlapactor))
        (Default|ShigtLever _asbp_lever))
      (:else))))

(event EventBeginPlay
  (bind _asbp_my_game_instance (Utilities|Casting|CastToBP_MyGameInstance (Game|GetGameInstance)))
  (Variables|Default|SetMyGameInstance_0 _asbp_my_game_instance)
  (bind _returnvalue (UserInterface|CreateWidget "/Game/Projects/Assets/UI/UW_GameUI.UW_GameUI_C"))
  (bind _output_get (Variables|Default|SetGameUI_0 _returnvalue))
  (UserInterface|Viewport|AddtoViewport _output_get 0)
  (CallFunction|InitializeKeyStatus)
  (Default|SetMessageFalse (Variables|Default|GetGameUI_0)))

(event EventControllerChanged
  (params (OldController :type Controller%20Object%20Reference) (NewController :type Controller%20Object%20Reference))
  (bind _asプレイヤーコントローラー (Utilities|Casting|CastToPlayerController NewController))
  (Input|AddMappingContext (PlayerController|LocalPlayerSubsystems|GetEnhancedInputLocalPlayerSubsystem _asプレイヤーコントローラー) "/Game/Projects/IMC_MyDefault.IMC_MyDefault" 0 "(bIgnoreAllPressedKeysUntilRelease=True,bForceImmediately=False,bNotifyUserSettings=False)"))

(event EventDestroyed
  (bind _returnvalue (Game|GetCurrentLevelName true))
  (Game|OpenLevel(byName) (Utilities|String|StringToName _returnvalue)))

(fn ConstructionScript
  (|CallParentFunction))

(fn InitializeKeyStatus
  (if (Utilities|Map|IsEmpty (Variables|/Game/Projects/Blueprints/BP_MyGameInstance.BP_MyGameInstance_C|GetKeyStatus (Variables|Default|GetMyGameInstance_0)))
    (bind _outrownames (DataTable|GetDataTableRowNames "/Game/Projects/Blueprints/DT_KeyStatus.DT_KeyStatus"))
    (for _array_element _outrownames
      (bind _returnvalue (Utilities|GetDataTableRow "/Game/Projects/Blueprints/DT_KeyStatus.DT_KeyStatus" _array_element)
        (:then
          (Default|SaveKeyStatus (Variables|Default|GetMyGameInstance_0) (.KeyName (Utilities|Struct|BreakST_KeyStatus _returnvalue)) (.KeyStatus (Utilities|Struct|BreakST_KeyStatus _returnvalue))))))))

(fn UpdateMessage
  (bind _returnvalue (Utilities|Text|MakeLiteralText "今は開かない"))
  (bind _overlapactor (Variables|Default|GetOverlapActor)
    (:then
      (bind _asbp_door (Utilities|Casting|CastToBP_Door _overlapactor)
        (:then
          (if (== (Variables|/Game/Projects/Blueprints/BP_Door.BP_Door_C|GetKeyName _asbp_door) "")
            (if (Variables|/Game/Projects/Blueprints/BP_Door.BP_Door_C|GetSwitchDoor _asbp_door)
              (Default|SetDisplayMessage (Variables|Default|GetGameUI_0) _returnvalue))
            (else
              (switch Utilities|FlowControl|Switch|SwitchonEN_KeyStatus (Default|GetKeyStatus (Variables|Default|GetMyGameInstance_0) (Variables|/Game/Projects/Blueprints/BP_Door.BP_Door_C|GetKeyName _asbp_door))
                (:NewEnumerator0
                  (Default|SetDisplayMessage (Variables|Default|GetGameUI_0) _returnvalue))
                (:NewEnumerator1
                  (Default|SetDisplayMessage (Variables|Default|GetGameUI_0) :!label _label))
                (:NewEnumerator2
                  (goto _label))))))
        (:CastFailed
          (Utilities|Casting|CastToBP_Lever (Variables|Default|GetOverlapActor)
            (:then
              (Default|SetDisplayMessage (Variables|Default|GetGameUI_0) "左クリック:レバーを引く"))
            (:CastFailed
              (Default|SetDisplayMessage (Variables|Default|GetGameUI_0)))))))
    (:else
      (Default|SetDisplayMessage (Variables|Default|GetGameUI_0)))))

(fn CharactorDeadEvent
  (|CallParentFunction)
  (Default|SetDisplayCenterMessage (Variables|Default|GetGameUI_0) false))

(fn CharactorGoalEvent
  (|CallParentFunction)
  (Default|SetDisplayGoalMessage (Variables|Default|GetGameUI_0) false))