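; BP_MyCharactor is a character Blueprint that manages HP, death and goal completion.
; CurrentHP starts at MaxHP in the construction script; AnyDamage reduces it and broadcasts OnCharacterHpChanged.
; At zero HP or below, the death event disables input, turns the mesh into a physics ragdoll and sets a short lifespan.
; The goal event disables input, calls the game UI's goal-message setter and also sets a short lifespan.
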(event Game|Damage|EventAnyDamage
  (params (Damage :type Float%20%28single-precision%29) (DamageType :type Damage%20Type%20Object%20Reference) (InstigatedBy :type Controller%20Object%20Reference) (DamageCauser :type Actor%20Object%20Reference))
  (bind _output_get (Variables|Default|SetCurrentHP (- (Variables|Default|GetCurrentHP) Damage)))
  (Default|CallOnCharacterHpChanged (Variables|Default|GetMaxHP) _output_get)
  (if (<= _output_get 0.0)
    (CallFunction|CharactorDeadEvent)))

(fn ConstructionScript
  (Variables|Default|SetCurrentHP (Variables|Default|GetMaxHP)))

(fn CharactorDeadEvent
  (bind _mesh (Variables|Character|GetMesh))
  (Input|DisableInput 0)
  (Collision|SetCollisionProfileName _mesh "Ragdoll" true :!class /Script/Engine.PrimitiveComponent)
  (Physics|SetSimulatePhysics _mesh true)
  (Actor|SetLifeSpan 3.0))

(fn CharactorGoalEvent
  (Input|DisableInput 0)
  (Default|SetDisplayGoalMessage (Variables|Default|GetGameUI) false)
  (Actor|SetLifeSpan 2.0))