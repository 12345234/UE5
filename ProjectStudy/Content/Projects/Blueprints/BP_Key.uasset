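; BP_Key is a collectible key pickup that spins in place until the player touches it.
; On BeginPlay, the Rotation timeline drives the yaw of the STMKey mesh, leaving roll and pitch unchanged.
; When a BP_TestCharactor overlaps the Sphere, the key passes its KeyName and a new status to that character's UpdateKeyStatus, then destroys itself.
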(event OnComponentBeginOverlap(Sphere)
  (params (OverlappedComponent :type Primitive%20Component%20Object%20Reference) (OtherActor :type Actor%20Object%20Reference) (OtherComp :type Primitive%20Component%20Object%20Reference) (OtherBodyIndex :type Integer) (bFromSweep :type Boolean) (SweepResult :type Hit%20Result%20Structure%20%28by%20ref%29))
  ;[0.15 0.15 0.15 0.5] 当たり判定(プレイヤーに当たると消える)
  (bind _asbp_test_charactor (Utilities|Casting|CastToBP_TestCharactor OtherActor))
  (Default|UpdateKeyStatus _asbp_test_charactor (Variables|Default|GetKeyName) "NewEnumerator1")
  (Actor|DestroyActor))

(event EventBeginPlay
  (bind _stm_key (Variables|Default|GetSTM_Key))
  (bind _relativerotation (Variables|/Script/Engine.SceneComponent|GetRelativeRotation _stm_key))
  (bind (_roll _pitch) (Math|Rotator|BreakRotator _relativerotation))
  ;[0.15 0.15 0.15 0.5] オブジェクトの回転
  (bind _rotationz (Timeline|Rotation Play)
    (:Update
      (Transformation|SetRelativeRotation (Variables|Default|GetSTM_Key) (Math|Rotator|MakeRotator _roll _pitch _rotationz) false false))))

(fn ConstructionScript)