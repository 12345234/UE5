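; BP_Door is a door actor that swings open when a BP_TestCharactor enters its box trigger, optionally requiring a key.
; With no KeyName set it opens directly; otherwise it opens only if the character's status for that key is Got, then marks it Used.
; A timeline drives the STMDoor mesh's yaw to animate the opening.
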(event OnComponentBeginOverlap(Box)
  (params (OverlappedComponent :type Primitive%20Component%20Object%20Reference) (OtherActor :type Actor%20Object%20Reference) (OtherComp :type Primitive%20Component%20Object%20Reference) (OtherBodyIndex :type Integer) (bFromSweep :type Boolean) (SweepResult :type Hit%20Result%20Structure%20%28by%20ref%29))
  (bind _keyname (Variables|Default|GetKeyName))
  (bind _asbp_test_charactor (Utilities|Casting|CastToBP_TestCharactor OtherActor))
  (if (== _keyname "")
    (bind _openz (Timeline|タイムライン Play)
      (:Update
        (Transformation|SetRelativeRotation (Variables|Default|GetSTM_Door) (Math|Rotator|MakeRotator 0.0 0.0 _openz) false false)))
    (else
      (switch Utilities|FlowControl|Switch|SwitchonEN_KeyStatus (Default|GetKeyStatus _asbp_test_charactor _keyname)
        (:NewEnumerator1
          (Default|UpdateKeyStatus _asbp_test_charactor (Variables|Default|GetKeyName) "NewEnumerator2")
          (Timeline|タイムライン Play))))))

(fn ConstructionScript)